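; BP_BasicCharacter is a character Blueprint that turns to face its horizontal direction of travel, as used for sprite rotation.
; Each Tick calls the parent, then checks the sign of the movement component's X velocity.
; A valid controller's control rotation snaps to yaw 0 for rightward or 180 for leftward movement.
; At zero X velocity the rotation is left unchanged, so the last facing persists.
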(event `self.ReceiveTick`
  (params (DeltaSeconds :type "Float (single-precision)"))
  (bind _returnvalue (`self.GetController`))
  (bind _returnvalue_2 (`self.GetController`))
  ;[0.133 1 0.2084] Sprite Rotation
  (`parent.ReceiveTick` DeltaSeconds)
  (`/Engine/EditorBlueprintResources/StandardMacros.CompareFloat` (.x (`MovementComponent.Velocity` (`self.GetMovementComponent`)))
    (:`>`
      ;;[0 0.4745 1] Look Right
      (`/Engine/EditorBlueprintResources/StandardMacros.IsValid` _returnvalue_2
        (:`Is Valid`
          (`Controller.SetControlRotation` _returnvalue_2 (`KismetMathLibrary.MakeRotator` 0.0)))))
    (:`<`
      ;;[0 0.4745 1] Look Left
      (`/Engine/EditorBlueprintResources/StandardMacros.IsValid` _returnvalue
        (:`Is Valid`
          (`Controller.SetControlRotation` _returnvalue (`KismetMathLibrary.MakeRotator` 0.0 0.0 180.0)))))))

(fn `UserConstructionScript`)