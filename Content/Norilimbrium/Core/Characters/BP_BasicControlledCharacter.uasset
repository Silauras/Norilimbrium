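; BP_BasicControlledCharacter is a controlled character Blueprint that provides camera zoom through its SpringArm.
; ChangeCameraDistance takes a camera input and sets the arm length through a math expression.
; The step is the input scaled by the natural log of the current length, so zoom moves faster when farther out, clamped between minimum and maximum camera distances.
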(fn ConstructionScript)

(fn ChangeCameraDistance
  (params (MoveCameraInput :type Float%20%28double-precision%29))
  (Variables|/Script/Engine.SpringArmComponent|SetTargetArmLength (Variables|Default|GetSpringArm) (|(Clamp((ArmLength+(MoveCameraInput*(Loge(ArmLength)))),{B859CA44-4287-59A2-AFE0-15A70EAD2D11},{2F9E1B59-495E-8963-E906-88A64972ABB8})) MoveCameraInput (Variables|/Script/Engine.SpringArmComponent|GetTargetArmLength (Variables|Default|GetSpringArm)))))